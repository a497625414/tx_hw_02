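; A flying target actor that moves in a straight line and can be shot down for score.
; Tick offsets the actor from the Cube's transform along Direction by Speed and delta time; a delayed FlipFlop resets Direction, but both branches set the same vector.
; A BP_Projectile hit on the Sphere destroys the actor, increments the first player's MyPlayerState score and asks MyGameMode to respawn that player.
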(event OnComponentHit(Sphere)
  (params (HitComponent :type Primitive%20Component%20Object%20Reference) (OtherActor :type Actor%20Object%20Reference) (OtherComp :type Primitive%20Component%20Object%20Reference) (NormalImpulse :type Vector :default "0, 0, 0") (Hit :type Hit%20Result%20Structure%20%28by%20ref%29))
  (bind _returnvalue (Game|GetPlayerController 0))
  (bind _playerstate (Variables|/Script/Engine.Controller|GetPlayerState _returnvalue))
  (bind _asbp_projectile (Utilities|Casting|CastToBP_Projectile OtherActor))
  (Actor|DestroyActor)
  (bind _asmy_player_state (Utilities|Casting|CastToMyPlayerState _playerstate)
    (:then
      (Default|IncrementScore _asmy_player_state))
    (:CastFailed
      _))
  (bind _asmy_game_mode (Utilities|Casting|CastToMyGameMode (Game|GetGameMode)))
  (bind _asplayer_controller (Utilities|Casting|CastToPlayerController (Pawn|GetController (Game|Player|GetPlayerPawn 0))))
  (Default|RespawnPlayerEvent _asmy_game_mode _asplayer_controller)
  (Development|PrintString (Utilities|GetDisplayName _playerstate) true true "(R=0.000000,G=0.660000,B=1.000000,A=1.000000)" 1e+01))

(event OnComponentHit(Cube)
  (params (HitComponent :type Primitive%20Component%20Object%20Reference) (OtherActor :type Actor%20Object%20Reference) (OtherComp :type Primitive%20Component%20Object%20Reference) (NormalImpulse :type Vector :default "0, 0, 0") (Hit :type Hit%20Result%20Structure%20%28by%20ref%29)))

(event EventBeginPlay)

(event Collision|EventActorBeginOverlap
  (params (OtherActor :type Actor%20Object%20Reference)))

(event EventTick
  (params (DeltaSeconds :type Float%20%28single-precision%29))
  (bind _cube (Variables|Default|GetCube))
  (bind _returnvalue (Transformation|GetWorldTransform _cube))
  (bind (_location _rotation _scale) (Math|Transform|BreakTransform _returnvalue))
  (Transformation|SetActorTransform (Math|Transform|MakeTransform (+ (* (Math|Vector|Normalize (Variables|Default|Getdirection)) (* (Utilities|Time|GetWorldDeltaSeconds) (Variables|Default|Getspeed))) _location) _rotation _scale))
  (Utilities|FlowControl|Delay 5.0)
  (Utilities|FlowControl|FlipFlop
    (:A
      (Variables|Default|Setdirection "-10.000000, 0, 0"))
    (:B
      (Variables|Default|Setdirection "-10.000000, 0, 0"))))

(fn ConstructionScript)