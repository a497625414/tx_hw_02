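; MyGameState runs the match countdown and opens the end-of-game settlement screen.
; On BeginPlay it adds the Daojishi (countdown) widget to the viewport, then decrements Gametime once per second through a looping Delay.
; When Gametime drops below one, it waits another second and adds the Jiesuanmianban (settlement panel) widget.
; The RepNotify handlers for GameStartTimer and RandomTimerValue1 are empty.
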(event EventBeginPlay
  (bind _returnvalue (UserInterface|CreateWidget "/Game/Blueprints/Widgets/daojishi.daojishi_C"))
  (bind _output_get (Variables|Default|SetdaojishiReference _returnvalue))
  (UserInterface|Viewport|AddtoViewport _output_get 0)
  (if (>= (Variables|Default|GetGametime) 1) :!label _label
    (Utilities|FlowControl|Delay 1.0)
    (Variables|Default|SetGametime (- (Variables|Default|GetGametime) 1))
    (goto _label)
    (else
      (Utilities|FlowControl|Delay 1.0)
      (bind _returnvalue_2 (UserInterface|CreateWidget "/Game/Blueprints/Widgets/jiesuanmianban.jiesuanmianban_C"))
      (bind _output_get_2 (Variables|Default|Setjiesuanmianban _returnvalue_2))
      (UserInterface|Viewport|AddtoViewport _output_get_2 0))))

(fn ConstructionScript)

(fn OnRepGameStartTimer)

(fn OnRepRandomTimerValue1)